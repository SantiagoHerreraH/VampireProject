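; Player character Blueprint that drives a projectile manager and applies damage over time through its life component.
; Tick updates projectile behaviour and, while damage over time is active, reduces life via a Delay-paced check; releasing T advances the projectile at index 0 a level.
; SetProjectileGrowthType maps simple pattern names to manager growth types.
; KillPlayerAndSpawn ragdolls, then teleports to a random reachable point, but its call here is unconnected.
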(event `KillPlayerAndSpawn`
  (bind _returnvalue (`GameplayStatics.GetPlayerController` 0))
  ;[0.2477 0 1] KillRoutine
  (`PrimitiveComponent.SetSimulatePhysics` (`self.Mesh`) true)
  (`self.DisableInput` _returnvalue)
  (`KismetSystemLibrary.Delay` 1.0)
  (`self.K2_SetActorLocation` (`NavigationSystemV1.K2_GetRandomReachablePointInRadius` (`self.K2_GetActorLocation`) 0.0 null null) false true)
  (`PrimitiveComponent.SetSimulatePhysics` (`self.Mesh`) false)
  (`self.EnableInput` _returnvalue))

(event `self.ReceiveTick`
  (params (DeltaSeconds :type "Float (single-precision)"))
  (bind _m_lifecomponent (`self.m_LifeComponent`))
  (bind _isdamageovertime (`LifeComponent.isDamageOverTime` _m_lifecomponent))
  ;[1 0 0.229] ProjectileBehaviour
  (`ProjectileManagerComponent.UpdateProjectileBehaviour` (`self.MProjectileManager`))
  ;[0 1 0.5165] CheckLife
  (if _isdamageovertime
    (`KismetSystemLibrary.Delay` (`LifeComponent.timeBetweenTicks` _m_lifecomponent))
    (if _isdamageovertime
      (`self.ReduceLife` (`LifeComponent.damagePerTick` _m_lifecomponent)))))

(event `Key|T`
  (params (Key :type "Key Structure"))
  (:`Released`
    (`ProjectileManagerComponent.NextLevel` (`self.MProjectileManager`) 0)))

(fn `SetProjectileGrowthType`
  (params (Type :type "/Game/Types/ProjectileGrowthTypes/ProjectileGrowthTypes_ENUM Enum" :default "NewEnumerator0"))
  (switch `/Game/Types/ProjectileGrowthTypes/ProjectileGrowthTypes_ENUM` Type
    (:`NewEnumerator0`
      (`ProjectileManagerComponent.SetProjectileGrowthType` (`self.MProjectileManager`) "/Game/Types/ProjectileGrowthTypes/StarSpreadStraight_3To12Directions_NonRel_Normal.StarSpreadStraight_3To12Directions_NonRel_Normal" 0))
    (:`NewEnumerator1`
      (`ProjectileManagerComponent.SetProjectileGrowthType` (`self.MProjectileManager`) "/Game/Types/ProjectileGrowthTypes/StraightForward_1To13Directions_Relative_NormalProjectile.StraightForward_1To13Directions_Relative_NormalProjectile" 0))
    (:`NewEnumerator2`
      (`ProjectileManagerComponent.SetProjectileGrowthType` (`self.MProjectileManager`) "/Game/Types/ProjectileGrowthTypes/VertStraight_1To5Directions_Relative_NormalProjectile.VertStraight_1To5Directions_Relative_NormalProjectile" 0))
    (:`NewEnumerator3`
      (`ProjectileManagerComponent.SetProjectileGrowthType` (`self.MProjectileManager`) "/Game/Types/ProjectileGrowthTypes/SpiralStar_1To5Directions_RelativeAndNon_NormalProjectile.SpiralStar_1To5Directions_RelativeAndNon_NormalProjectile" 0))
    (:`NewEnumerator4`
      (`ProjectileManagerComponent.SetProjectileGrowthType` (`self.MProjectileManager`) "/Game/Types/ProjectileGrowthTypes/DomeStraight_3To9Directions_Relative_NormalProjectile.DomeStraight_3To9Directions_Relative_NormalProjectile" 0))))

(fn `UserConstructionScript`)