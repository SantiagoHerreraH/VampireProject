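; BP_FirstAidKitItem is a first aid kit pickup that heals the player character.
; It initializes on BeginPlay with a recovery amount and uses a small collider, sized in the construction script, to detect overlaps.
; When BP_ProyectoVampiroCharacter overlaps and its life component is below max, it sends RestoreLifeMessage with LifeRecovered and destroys itself, so full-health characters leave it in place.
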(event `self.ReceiveBeginPlay`
  (`self.Init` 25.0))

(event `self.BoxCollider.OnComponentBeginOverlap`
  (params (OverlappedComponent :type "PrimitiveComponent Object Reference") (OtherActor :type "Actor Object Reference") (OtherComp :type "PrimitiveComponent Object Reference") (OtherBodyIndex :type Integer) (bFromSweep :type Boolean) (SweepResult :type "HitResult Structure (by ref)"))
  (bind _asbp_proyecto_vampiro_character (cast `/Game/Blueprints/BP_ProyectoVampiroCharacter` OtherActor))
  (bind _m_lifecomponent (`ProyectoVampiroCharacter.m_LifeComponent` _asbp_proyecto_vampiro_character))
  (`/Engine/EditorBlueprintResources/StandardMacros.IsValid` _m_lifecomponent
    (:`Is Valid`
      (if (!= (`LifeComponent.currentLife` _m_lifecomponent) (`LifeComponent.maxLife` _m_lifecomponent))
        (message `LifeManagerInterface.RestoreLife` _asbp_proyecto_vampiro_character (`self.LifeRecovered`))
        (`self.K2_DestroyActor`)))))

(fn `UserConstructionScript`
  (`SphereComponent.SetSphereRadius` (`self.BoxCollider`) 25.0 true))