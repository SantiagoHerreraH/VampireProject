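; Pickup item that switches the player character's projectile growth type when touched.
; BeginPlay derives the growth type from the enum's entry count minus one and requests a spawn of its class from the game instance's spawn pool.
; On overlap with the player, it applies that type, then despawns and respawns through the pool.
; Spawn locations are random reachable navigation points around the item's position.
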(event `self.ReceiveBeginPlay`
  (set `self.GrowthType` (cast `/Game/Types/ProjectileGrowthTypes/ProjectileGrowthTypes_ENUM` (`KismetMathLibrary.Conv_IntToByte` (- (enumcount `/Game/Types/ProjectileGrowthTypes/ProjectileGrowthTypes_ENUM`) 1))))
  (bind _asvampire_game_instance (cast `VampireGameInstance` (`GameplayStatics.GetGameInstance`)))
  (bind _returnvalue (`VampireGameInstance.GetSpawnPool` _asvampire_game_instance))
  (`SpawnPool.SpawnActor` :`self` _returnvalue :`classType` (`GameplayStatics.GetObjectClass` self) :`spawnLocation` (`NavigationSystemV1.K2_GetRandomReachablePointInRadius` (`self.K2_GetActorLocation`) 0.0 null null) :`spawnedActorScale` (1.0 1.0 1.0)))

(event `self.BoxCollider.OnComponentBeginOverlap`
  (params (OverlappedComponent :type "PrimitiveComponent Object Reference") (OtherActor :type "Actor Object Reference") (OtherComp :type "PrimitiveComponent Object Reference") (OtherBodyIndex :type Integer) (bFromSweep :type Boolean) (SweepResult :type "HitResult Structure (by ref)"))
  (bind _returnvalue (`GameplayStatics.GetObjectClass` self))
  (bind _asbp_proyecto_vampiro_character (cast `/Game/Blueprints/BP_ProyectoVampiroCharacter` OtherActor))
  (`/Game/Blueprints/BP_ProyectoVampiroCharacter.SetProjectileGrowthType` _asbp_proyecto_vampiro_character (`self.GrowthType`))
  (bind _asvampire_game_instance (cast `VampireGameInstance` (`GameplayStatics.GetGameInstance`)))
  (bind _returnvalue_2 (`VampireGameInstance.GetSpawnPool` _asvampire_game_instance))
  (`SpawnPool.DespawnActor` _returnvalue_2 null _returnvalue)
  (`SpawnPool.SpawnActor` :`self` _returnvalue_2 :`actor` self :`classType` _returnvalue :`spawnLocation` (`NavigationSystemV1.K2_GetRandomReachablePointInRadius` (`self.K2_GetActorLocation`) 0.0 null null) :`spawnedActorScale` (1.0 1.0 1.0)))

(fn `UserConstructionScript`
  (`SphereComponent.SetSphereRadius` (`self.BoxCollider`) 25.0 true))