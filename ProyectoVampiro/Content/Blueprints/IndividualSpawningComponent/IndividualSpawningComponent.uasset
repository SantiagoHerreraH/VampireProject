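; Actor component that spawns and despawns its owning actor through the shared spawn pool held by VampireGameInstance.
; Spawn places the owner at a given location, while SpawnRandom picks a reachable navmesh point within a radius of the owner's current position.
; Despawn hands the owner back to the pool, with every call keyed by the owner's class.
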(event `Spawn`
  (params (SpawnLocation :type "Vector Structure"))
  (bind _returnvalue (`self.GetOwner`))
  (bind _asvampire_game_instance (cast `VampireGameInstance` (`GameplayStatics.GetGameInstance`)))
  (bind _returnvalue_2 (`VampireGameInstance.GetSpawnPool` _asvampire_game_instance))
  (`SpawnPool.SpawnActor` :`self` _returnvalue_2 :`actor` _returnvalue :`classType` (`GameplayStatics.GetObjectClass` _returnvalue) :`spawnLocation` SpawnLocation :`spawnedActorScale` (1.0 1.0 1.0)))

(event `SpawnRandom`
  (bind _returnvalue (`self.GetOwner`))
  (bind _asvampire_game_instance (cast `VampireGameInstance` (`GameplayStatics.GetGameInstance`)))
  (bind _returnvalue_2 (`VampireGameInstance.GetSpawnPool` _asvampire_game_instance))
  (`SpawnPool.SpawnActor` :`self` _returnvalue_2 :`actor` _returnvalue :`classType` (`GameplayStatics.GetObjectClass` _returnvalue) :`spawnLocation` (`NavigationSystemV1.K2_GetRandomReachablePointInRadius` (`Actor.K2_GetActorLocation` _returnvalue) 3000.0 null null) :`spawnedActorScale` (1.0 1.0 1.0)))

(event `Despawn`
  (bind _returnvalue (`self.GetOwner`))
  (bind _asvampire_game_instance (cast `VampireGameInstance` (`GameplayStatics.GetGameInstance`)))
  (bind _returnvalue_2 (`VampireGameInstance.GetSpawnPool` _asvampire_game_instance))
  (`SpawnPool.DespawnActor` _returnvalue_2 _returnvalue (`GameplayStatics.GetObjectClass` _returnvalue)))